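; BP_Enemy is a spinning enemy that the player can shoot for points or collide with for damage.
; RandomizeEnemy randomly either keeps it, setting a cone mesh and jittering its position, or destroys it, and returns the result.
; A BP_Bullet overlap increments Score through the bullet's player reference and destroys the enemy.
; A mesh hit on BP_Player shakes the camera, deducts clamped health, destroys the enemy and shows restart at zero.
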(event `self.ReceiveTick`
  (params (DeltaSeconds :type "Float (single-precision)"))
  (`self.K2_AddActorLocalRotation` (`KismetMathLibrary.MakeRotator` (* DeltaSeconds (`self.RotateSpeed`)))))

(event `self.ReceiveActorBeginOverlap`
  (params (OtherActor :type "Actor Object Reference"))
  (bind _asbp_bullet (cast `/Game/InfiniteMatrix/Blueprints/BP_Bullet` OtherActor)) ; Make the enemy disappear if a projectile hits it.
  (bind _playerreference (`/Game/InfiniteMatrix/Blueprints/BP_Bullet.PlayerReference` _asbp_bullet))
  (set `/Game/InfiniteMatrix/Blueprints/BP_Player.Score` (+ (`/Game/InfiniteMatrix/Blueprints/BP_Player.Score` _playerreference) 1) _playerreference)
  (`self.K2_DestroyActor`))

(event `self.EnemyMesh.OnComponentHit`
  (params (HitComponent :type "PrimitiveComponent Object Reference") (OtherActor :type "Actor Object Reference") (OtherComp :type "PrimitiveComponent Object Reference") (NormalImpulse :type "Vector Structure") (Hit :type "HitResult Structure (by ref)"))
  (bind _asbp_player (cast `/Game/InfiniteMatrix/Blueprints/BP_Player` OtherActor)) ; Check that the actor that the wall collided with is the player.
  (`GameplayStatics.PlayWorldCameraShake` "/Game/InfiniteMatrix/Blueprints/BP_CameraShake.BP_CameraShake_C" (`self.K2_GetActorLocation`) 0.0 2000.0)
  (bind _output_get (set `/Game/InfiniteMatrix/Blueprints/BP_Player.Health` (`KismetMathLibrary.FClamp` (- (`/Game/InfiniteMatrix/Blueprints/BP_Player.Health` _asbp_player) 10.0) 0.0 100.0) _asbp_player))
  (`self.K2_DestroyActor`) ; Destroy the enemy after hitting it.
  (if (== _output_get 0.0)
    (`/Game/InfiniteMatrix/Blueprints/BP_Player.DisplayRestart` _asbp_player) ; Call the display restart button after the user collides with the wall.
  ))

(fn `RandomizeEnemy`
  (returns (EnemySpawned :type Boolean))
  (if (> (`KismetMathLibrary.RandomIntegerInRange` 0 9) 2)
    (`StaticMeshComponent.SetStaticMesh` (`self.EnemyMesh`) "/Engine/BasicShapes/Cone.Cone")
    (`self.K2_AddActorLocalOffset` (`KismetMathLibrary.MakeVector` (`KismetMathLibrary.RandomFloatInRange` -400.0 400.0) (`KismetMathLibrary.RandomFloatInRange` -400.0 400.0) (`KismetMathLibrary.RandomFloatInRange` -200.0 200.0))) ; Randomize the location of the next enemy. Determined coordinates from seeing which coordinates allow enemy to show up.
    (return true)
    (else
      (`self.K2_DestroyActor`)
      (return false))))

(fn `UserConstructionScript`)