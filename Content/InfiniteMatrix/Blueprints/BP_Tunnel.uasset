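; BP_Tunnel is an endless-runner tunnel segment with a spinning holed wall and an optional healthpack.
; Randomize functions pick the wall mesh and angle and decide healthpack presence and placement, while Tick rotates both.
; Passing the trigger adds score and periodically boosts player speed; wall hits cost health and show restart at zero, and healthpack hits heal.
; Passing or hitting the wall has TunnelSpawner spawn the next segment and destroys this one.
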(event `self.ReceiveTick`
  (params (DeltaSeconds :type "Float (single-precision)"))
  (bind _rotatespeed (`self.RotateSpeed`))
  (`SceneComponent.K2_AddLocalRotation` (`self.WallMesh`) (`KismetMathLibrary.MakeRotator` (* DeltaSeconds _rotatespeed)) false false) ; Makes wall mesh rotate every frame by the specified amount
  (`/Engine/EditorBlueprintResources/StandardMacros.IsValid` (`self.HealthpackMesh`) ; Rotate the healthpack around as well.
    (:`Is Valid`
      (`SceneComponent.K2_AddLocalRotation` (`self.HealthpackMesh`) (`KismetMathLibrary.MakeRotator` (* DeltaSeconds _rotatespeed)) false false))))

(event `self.TriggerZone.OnComponentBeginOverlap`
  (params (OverlappedComponent :type "PrimitiveComponent Object Reference") (OtherActor :type "Actor Object Reference") (OtherComp :type "PrimitiveComponent Object Reference") (OtherBodyIndex :type Integer) (bFromSweep :type Boolean) (SweepResult :type "HitResult Structure (by ref)"))
  (bind _asbp_player (cast `/Game/InfiniteMatrix/Blueprints/BP_Player` OtherActor)) ; Ensures that further nodes only executes if the actor is the player
  (`/Game/InfiniteMatrix/Blueprints/BP_TunnelSpawner.SpawnTunnelAtSpawnPoint` (`self.TunnelSpawner`)) ; Spawn new tunnel at the spawn point of the last tunnel
  (`self.K2_DestroyActor`) ; Remove the old tunnel since we don't need it anymore
  (set `/Game/InfiniteMatrix/Blueprints/BP_Player.Score` (+ (`/Game/InfiniteMatrix/Blueprints/BP_Player.Score` _asbp_player) 1) _asbp_player) ; Increase the score of the player by one after passing the trigger zone.
  (bind _score (`/Game/InfiniteMatrix/Blueprints/BP_Player.Score` _asbp_player))
  (if (and (== (mod _score 5) 0) (> _score 1))
    (bind _output_get (set `/Game/InfiniteMatrix/Blueprints/BP_Player.ForwardSpeed` (* (`/Game/InfiniteMatrix/Blueprints/BP_Player.ForwardSpeed` _asbp_player) 1.1) _asbp_player))
    (`KismetSystemLibrary.PrintText` (`KismetTextLibrary.Conv_DoubleToText` _output_get "HalfToEven"))))

(event `self.WallMesh.OnComponentHit`
  (params (HitComponent :type "PrimitiveComponent Object Reference") (OtherActor :type "Actor Object Reference") (OtherComp :type "PrimitiveComponent Object Reference") (NormalImpulse :type "Vector Structure") (Hit :type "HitResult Structure (by ref)"))
  (bind _asbp_player (cast `/Game/InfiniteMatrix/Blueprints/BP_Player` OtherActor)) ; Check that the actor that the wall collided with is the player.
  (bind _output_get (set `/Game/InfiniteMatrix/Blueprints/BP_Player.Health` (`KismetMathLibrary.FClamp` (- (`/Game/InfiniteMatrix/Blueprints/BP_Player.Health` _asbp_player) 10.0) 0.0 100.0) _asbp_player))
  (`/Game/InfiniteMatrix/Blueprints/BP_TunnelSpawner.SpawnTunnelAtSpawnPoint` (`self.TunnelSpawner`)) ; If we still have health after hitting the tunnel, then we just go through the tunnel, which is basically just destroying the tunnel.
  (`/Engine/EditorBlueprintResources/StandardMacros.IsValid` (`self.HealthpackMesh`) ; Delete the healthpack spawned in the tunnel if it still exists.
    (:`Is Valid`
      (`ActorComponent.K2_DestroyComponent` (`self.HealthpackMesh`)) ; Destroy the healthpack mesh after passing the tunnel.
    )
    (:`Is Not Valid`
      _))
  (`self.K2_DestroyActor`)
  (if (== _output_get 0.0)
    (`/Game/InfiniteMatrix/Blueprints/BP_Player.DisplayRestart` _asbp_player) ; Call the display restart button after the user collides with the wall.
  ))

(event `self.HealthpackMesh.OnComponentHit`
  (params (HitComponent :type "PrimitiveComponent Object Reference") (OtherActor :type "Actor Object Reference") (OtherComp :type "PrimitiveComponent Object Reference") (NormalImpulse :type "Vector Structure") (Hit :type "HitResult Structure (by ref)"))
  (bind _asbp_player (cast `/Game/InfiniteMatrix/Blueprints/BP_Player` OtherActor)) ; Check that the actor that the wall collided with is the player.
  (set `/Game/InfiniteMatrix/Blueprints/BP_Player.Health` (`KismetMathLibrary.FClamp` (+ (`/Game/InfiniteMatrix/Blueprints/BP_Player.Health` _asbp_player) 10.0) 0.0 100.0) _asbp_player)
  (`ActorComponent.K2_DestroyComponent` (`self.HealthpackMesh`)) ; Destroy the healthpack mesh after using it.
)

(fn `Randomize Health Pack`
  (if (> (`KismetMathLibrary.RandomIntegerInRange` 0 9) 4)
    (`StaticMeshComponent.SetStaticMesh` (`self.HealthpackMesh`) "/Engine/VREditor/BasicMeshes/SM_Cube_02.SM_Cube_02")
    (`SceneComponent.K2_AddLocalOffset` (`self.HealthpackMesh`) (`KismetMathLibrary.MakeVector` (`KismetMathLibrary.RandomFloatInRange` -400.0 400.0) (`KismetMathLibrary.RandomFloatInRange` -400.0 400.0) (`KismetMathLibrary.RandomFloatInRange` -200.0 200.0)) false false) ; Randomize the location of the next health pack. Determined coordinates from seeing which coordinates allow health pack to show up.
    (else
      (`ActorComponent.K2_DestroyComponent` (`self.HealthpackMesh`)))))

(fn `RandomizeWall`
  (`StaticMeshComponent.SetStaticMesh` (`self.WallMesh`) (select `int` (`KismetMathLibrary.RandomIntegerInRange` 0 3) :`0` "/Game/InfiniteMatrix/Meshes/SM_Hole_01.SM_Hole_01" :`1` "/Game/InfiniteMatrix/Meshes/SM_Hole_02.SM_Hole_02" :`2` "/Game/InfiniteMatrix/Meshes/SM_Hole_03.SM_Hole_03" :`3` "/Game/InfiniteMatrix/Meshes/SM_Hole_04.SM_Hole_04" :!type "StaticMesh Object Reference")) ; Sets wall mesh to the supplied mesh
  (`SceneComponent.K2_AddLocalRotation` (`self.WallMesh`) (`KismetMathLibrary.MakeRotator` (`KismetMathLibrary.RandomFloatInRange` 0.0 360.0)) false false) ; Sets rotation for the wall
)

(fn `UserConstructionScript`)