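; Tunnel spawner actor that builds the chain of BP_Tunnel segments the player moves through.
; On BeginPlay it destroys any existing tunnels, then spawns three: the first at the player pawn, each next at the newest tunnel's SpawnPoint.
; Each new tunnel becomes NewestTunnel, receives a reference back to the spawner, and randomizes its wall, health pack and enemy.
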(event `self.ReceiveBeginPlay`
  (`self.SpawnInitialTunnels`))

(fn `SpawnInitialTunnels`
  (`|ExecutionSequence`
    (:`then_0`
      (bind _outactors (`GameplayStatics.GetAllActorsOfClass` "/Game/InfiniteMatrix/Blueprints/BP_Tunnel.BP_Tunnel_C")) ; This sequence will get all the existing tunnels and remove them from the game.
      (for _array_element _outactors
        (`self.K2_DestroyActor` _array_element)))
    (:`then_1`
      (for _ (range 3)
        (`/Engine/EditorBlueprintResources/StandardMacros.IsValid` (`self.NewestTunnel`) ; Check if the newest tunnel has spawned. First check will always be not valid.
          (:`Is Valid`
            (`self.SpawnTunnelAtSpawnPoint`) ; Spawning subsequent tunnels (will be at spawn point of newest tunnel).
          )
          (:`Is Not Valid`
            (`self.SpawnTunnel` (`self.K2_GetActorLocation` (`GameplayStatics.GetPlayerPawn` 0))) ; Spawns a tunnel at the player's location if there is no tunnel that has spawned.
          ))))))

(fn `SpawnTunnel`
  (params (SpawnLocation :type "Vector Structure"))
  (bind _returnvalue (`|SpawnActorFromClass` "/Game/InfiniteMatrix/Blueprints/BP_Tunnel.BP_Tunnel_C" (`KismetMathLibrary.MakeTransform` SpawnLocation) "Undefined" "OverrideRootScale" null null))
  (bind _output_get (set `self.NewestTunnel` _returnvalue)) ; Reference to the furthest tunnel
  (set `/Game/InfiniteMatrix/Blueprints/BP_Tunnel.TunnelSpawner` self _output_get) ; Allows every tunnel to have a reference to the tunnel spawner
  (`/Game/InfiniteMatrix/Blueprints/BP_Tunnel.RandomizeWall` _output_get) ; Randomize the wall that's chosen by calling the randomize wall function that we created
  (`/Game/InfiniteMatrix/Blueprints/BP_Tunnel.Randomize Health Pack` _output_get) ; Randomize the spawn location of the next health pack.
  (`/Game/InfiniteMatrix/Blueprints/BP_Tunnel.RandomizeEnemy` _output_get) ; Randomize the spawn location of the next enemy.
)

(fn `SpawnTunnelAtSpawnPoint`
  (`self.SpawnTunnel` (`SceneComponent.K2_GetComponentLocation` (`/Game/InfiniteMatrix/Blueprints/BP_Tunnel.SpawnPoint` (`self.NewestTunnel`)))) ; Spawns a new tunnel at the location of the newest tunnel's spawn point
)

(fn `UserConstructionScript`)